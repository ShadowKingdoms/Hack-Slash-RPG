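; Wolf boss character with a player-teleport jump attack, meteor and breath skills, a highlight material swap and item drops.
; Player damage gets random variance and critical rolls, spawning floating text and lowering a temporary HP that a timeline animates on the boss HP bar.
; Breath uses a delayed-loop macro to spawn repeated effects from the skull socket.
; Death fades dynamic materials, increments the kill count, shows results and destroys the actor.
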(event EventMonsterBreathEffect
  (bind _mesh (Variables|Character|GetMesh))
  ;[1 1 1] Skill_3 Breath
  (Utilities|SpawnBreath 0.1 (> 15 (Variables|Default|GetiBreathCount))
    (:Loop%20Body
      (Game|SpawnActorfromClass "/Game/BluePrint/Ability/AI/SKill_3/BP_Breath_Effect.BP_Breath_Effect_C" (Math|Transform|MakeTransform (Transformation|GetSocketLocation _mesh "c_skull_01_x") (Transformation|GetSocketRotation _mesh "c_skull_01_x")) "Undefined" 0 0 0)
      (Variables|Default|SetiBreathCount (+ (Variables|Default|GetiBreathCount) 1)))
    (:Exit
      (Variables|Default|SetiBreathCount 0))))

(event EventDropPickupItem
  (Game|SpawnActorfromClass "/Game/BluePrint/Monster/BP_MonsterItemSpawner.BP_MonsterItemSpawner_C" (Math|Transform|MakeTransform (|GetSpawnLocation) (Transformation|GetActorRotation)) "Undefined" 0 0))

(event EventToggleBossHPBarWidget
  (params (bVisibility :type Boolean))
  (bind _boss_hpbar_widget (Variables|Default|GetBoss%20HPBar%20Widget))
  (if bVisibility
    (UserInterface|Viewport|AddtoViewport _boss_hpbar_widget -500)
    (Default|PlayAnimation _boss_hpbar_widget)))

(event EventMonsterJumpEffect
  ;[1 1 1] Skill_4 JumpAttack
  (Transformation|SetActorRotation "0.000000,180.000000, 0")
  (Transformation|SetActorLocation (Transformation|GetActorLocation (Game|Player|GetPlayerPawn 0)) false true)
  (Collision|SetCollisionProfileName (Variables|Default|GetCapsuleComponent) "BossFalling" true :!class /Script/Engine.PrimitiveComponent)
  (Game|SpawnActorfromClass "/Game/BluePrint/Ability/AI/SKill_4/BP_CircularSector_Rev.BP_CircularSector_Rev_C" (Transformation|GetActorLocation) "Undefined" 0 0))

(event EventMonsterMeteorEffect
  ;[1 1 1] Skill_2 Meteor
  (bind _returnvalue (Game|SpawnActorfromClass "/Game/BluePrint/Ability/AI/SKill_2/BP_Meteor.BP_Meteor_C" (Transformation|GetActorTransform) "Undefined" 0 0))
  (Variables|/Script/LostArc.AIAbilityComponent|SetMeteorActorRef (Variables|Default|GetAbilityComponent) _returnvalue))

(event EventMonsterExtinctionEffects
  (bind _mesh (Variables|Character|GetMesh))
  ;[1 1 1] Wolf Death
  (bind _foundwidgets (Widget|GetAllWidgetsOfClass "/Game/UI/Damage/BP_BossHPBar.BP_BossHPBar_C" true))
  (Widget|RemovefromParent _foundwidgets)
  (bind _returnvalue (Rendering|Material|CreateDynamicMaterialInstance _mesh 0 (Rendering|Material|GetMaterial _mesh 0) "None" :!class /Script/Engine.PrimitiveComponent))
  (bind _output_get (Variables|Default|SetM_ApperParmRef_0 _returnvalue))
  (bind _returnvalue_2 (Rendering|Material|CreateDynamicMaterialInstance _mesh 1 (Rendering|Material|GetMaterial _mesh 1) "None" :!class /Script/Engine.PrimitiveComponent))
  (bind _output_get_2 (Variables|Default|SetM_ApperParmRef_1 _returnvalue_2))
  (bind _returnvalue_3 (Rendering|Material|CreateDynamicMaterialInstance _mesh 2 (Rendering|Material|GetMaterial _mesh 2) "None" :!class /Script/Engine.PrimitiveComponent))
  (bind _output_get_3 (Variables|Default|SetM_ApperParmRef_2 _returnvalue_3))
  (bind _returnvalue_4 (Rendering|Material|CreateDynamicMaterialInstance _mesh 3 (Rendering|Material|GetMaterial _mesh 3) "None" :!class /Script/Engine.PrimitiveComponent))
  (bind _output_get_4 (Variables|Default|SetM_ApperParmRef_3 _returnvalue_4))
  (bind _alpha (Timeline|timeline Play)
    (:Update
      (Rendering|Material|SetScalarParameterValue _output_get "Apperance" _alpha :!class /Script/Engine.MaterialInstanceDynamic))
    (:Finished
      (bind _aslost_arc_game_instance (Utilities|Casting|CastToLostArcGameInstance (Game|GetGameInstance)))
      (Class|LostArcGameInstance|PlusKillCount _aslost_arc_game_instance)
      (Utilities|FlowControl|Delay 1.0)
      (bind _returnvalue_5 (UserInterface|CreateWidget "/Game/UI/Result/BP_GameResultWidget.BP_GameResultWidget_C"))
      (UserInterface|Viewport|AddtoViewport _returnvalue_5 0)
      (Actor|DestroyActor))))

(event Game|Damage|EventAnyDamage
  (params (Damage :type Float%20%28single-precision%29) (DamageType :type Damage%20Type%20Object%20Reference) (InstigatedBy :type Controller%20Object%20Reference) (DamageCauser :type Actor%20Object%20Reference))
  (bind _aslost_arc_player_character (Utilities|Casting|CastToLostArcPlayerCharacter DamageCauser))
  (bind _returnvalue (Class|LostArcCharacterStatComponent|GetCriticalRate (Variables|/Script/LostArc.LostArcPlayerCharacter|GetStatComponent _aslost_arc_player_character)))
  ;[1 1 1] Random이 Rate 값 보다 작으면 Critical!
  (if (< (Math|Random|RandomFloatinRange 0.0 1e+02) _returnvalue)
    (bind _output_get (Variables|Default|SetDamage (* (Math|Random|RandomFloatinRange 0.7 1.1) (* 2 Damage))))
    (CallFunction|HandleDamage _output_get true)
    (else
      (bind _output_get_2 (Variables|Default|SetDamage (* (Math|Random|RandomFloatinRange 0.7 1.1) Damage)))
      (CallFunction|HandleDamage _output_get_2 false)))
  (Variables|Default|SetMonsterTempHP (- (Variables|Default|GetMonsterHP) (Variables|Default|GetDamage)))
  (Audio|PlaySoundatLocation "/Game/Sounds/Effects/MonsterHit/MonsterHItSoundCue.MonsterHItSoundCue" (Transformation|GetActorLocation) (Transformation|GetActorRotation) 1.0 1.0 0.0 0 "/Game/Sounds/Effects/MonsterHit/HitSoundConcurrency.HitSoundConcurrency" 0))

(event EventMonsterHPChanged
  (bind _boss_hpbar_widget (Variables|Default|GetBoss%20HPBar%20Widget))
  (Utilities|IsValid _boss_hpbar_widget
    (:Is%20Valid
      (if (Variables|Default|GetBar%20has%20Running)
        (Variables|Default|SetMonsterHP (- (Variables|Default|GetMonsterHP) (- (Variables|Default|GetMonsterHP) (Variables|Default|GetMonsterTempHP))))
        (bind _alpha (Timeline|HPBar%20Timeline PlayFromStart)
          (:Update
            (Progress|SetPercent (Variables|/Game/UI/Damage/BP_BossHPBar.BP_BossHPBar_C|GetProgressBar _boss_hpbar_widget) (Math|Float|NormalizetoRange (Math|Float|Lerp (Variables|Default|GetMonsterHP) (Variables|Default|GetMonsterTempHP) _alpha) 0.0 (Variables|Default|GetMonsterMaxHP)))
            (Variables|Default|SetBar%20has%20Running true))
          (:Finished
            (Variables|Default|SetMonsterHP (Variables|Default|GetMonsterTempHP))
            (Variables|Default|SetBar%20has%20Running false)))
        (else
          (Timeline|HPBar%20Timeline PlayFromStart))))))

(event EventBeginPlay
  (bind _returnvalue (UserInterface|CreateWidget "/Game/UI/Damage/BP_BossHPBar.BP_BossHPBar_C"))
  (Variables|Default|SetBoss%20HPBar%20Widget _returnvalue))

(event EventBossMonsterHighlightEffect
  ;[1 1 1] Monster Mesh Highlight
  (if (Variables|Default|GetbIsAbsent)
    (Rendering|Material|SetMaterial (Variables|Character|GetMesh) 0 "/Game/MaterialFunctionCollection/Materials/Materials/Fresnel/MI_Fresnel_01.MI_Fresnel_01")
    (Rendering|Material|SetMaterial (Variables|Character|GetMesh) 1 "/Game/MaterialFunctionCollection/Materials/Materials/Fresnel/MI_Fresnel_01.MI_Fresnel_01")
    (Rendering|Material|SetMaterial (Variables|Character|GetMesh) 2 "/Game/MaterialFunctionCollection/Materials/Materials/Fresnel/MI_Fresnel_01.MI_Fresnel_01")
    (Rendering|Material|SetMaterial (Variables|Character|GetMesh) 3 "/Game/MaterialFunctionCollection/Materials/Materials/Fresnel/MI_Fresnel_01.MI_Fresnel_01")
    (else
      (Rendering|Material|SetMaterial (Variables|Character|GetMesh) 0 (Variables|Default|GetM_Wolf0))
      (Rendering|Material|SetMaterial (Variables|Character|GetMesh) 1 (Variables|Default|GetM_Wolf1))
      (Rendering|Material|SetMaterial (Variables|Character|GetMesh) 2 (Variables|Default|GetM_Wolf2))
      (Rendering|Material|SetMaterial (Variables|Character|GetMesh) 3 (Variables|Default|GetM_Wolf3)))))

(fn ConstructionScript
  (Variables|Default|SetMonsterStr 1e+01)
  (Variables|Default|SetBasicAttackRadius 1.2e+02)
  (Variables|Default|SetMonsterDetectRadius 1024.0)
  (Variables|Default|SetBasicAttackRange 5e+02)
  (bind _output_get (Variables|Default|SetMonsterHP 1024.0))
  (bind _output_get_2 (Variables|Default|SetMonsterMaxHP _output_get))
  (Variables|Default|SetMonsterTempHP _output_get_2)
  (Variables|Default|SetBar%20has%20Running false)
  (Variables|Default|SetMonsterRotateSpeed 128.0)
  (bind _output_get_3 (Variables|Default|SetMonsterSpeed 4e+02))
  (Variables|/Script/Engine.CharacterMovementComponent|SetMaxWalkSpeed (Variables|Character|GetCharacterMovement) _output_get_3)
  (Variables|Default|SetM_WeaknessMetrial "/Game/MaterialFunctionCollection/Materials/Materials/Fresnel/MI_Fresnel_01.MI_Fresnel_01"))

(fn MonsterBreath
  (bind _mesh (Variables|Character|GetMesh))
  (Game|SpawnActorfromClass "/Game/BluePrint/Ability/AI/SKill_3/BP_Breath_Effect.BP_Breath_Effect_C" (Math|Transform|MakeTransform (Transformation|GetSocketLocation _mesh "c_skull_01_x") (Transformation|GetSocketRotation _mesh "c_skull_01_x")) "Undefined" 0 0 0))

(fn HandleDamage
  (params (Damage :type Float%20%28single-precision%29) (Is%20Critical :type Boolean))
  (bind _returnvalue (Transformation|GetActorLocation))
  (bind _returnvalue_2 (Math|Random|RandomFloatinRange -6e+01 6e+01))
  (bind _returnvalue_3 (Math|Random|RandomFloatinRange 128.0 192.0))
  (bind _returnvalue_4 (Math|Random|RandomFloatinRange -25.0 25.0))
  (bind _returnvalue_5 (+ _returnvalue (Math|Vector|MakeVector _returnvalue_4 _returnvalue_2 _returnvalue_3)))
  (if Is%20Critical
    (Game|SpawnActorfromClass "/Game/BluePrint/Boss/BP_Critical_Hit_Impact_Boss.BP_Critical_Hit_Impact_Boss_C" (Math|Transform|MakeTransform (Transformation|GetSocketLocation (Variables|Character|GetMesh) "head_x") "0, 0, 0" "1,1,1") "Undefined" 0 0)
    (bind _returnvalue_6 (Game|SpawnActorfromClass "/Game/UI/Damage/BP_FloatingCriticalTextActor.BP_FloatingCriticalTextActor_C" (Math|Transform|MakeTransform _returnvalue_5 "0, 0, 0" "1,1,1") "Undefined" 0 0))
    (Default|InitializeFunc _returnvalue_6 (Utilities|Text|ToText(Float) Damage "HalfToEven" false true 1 324 0 0))
    (else
      (bind _returnvalue_7 (Game|SpawnActorfromClass "/Game/UI/Damage/BP_FloatingTextActor.BP_FloatingTextActor_C" (Math|Transform|MakeTransform _returnvalue_5 "0, 0, 0" "1,1,1") "Undefined" 0 0))
      (Default|InitializeFunc _returnvalue_7 (Utilities|Text|ToText(Float) Damage "HalfToEven" false true 1 324 0 0)))))