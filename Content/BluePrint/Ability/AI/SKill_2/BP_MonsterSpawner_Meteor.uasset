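; One-shot monster spawner actor for the AI meteor skill that occasionally leaves enemies around its location.
; On BeginPlay it passes a weighted random roll, waits a random delay, then spawns small random numbers of melee-or-base and ranged monster characters.
; Spawn X and Y come from separate random navmesh queries nearby, with Z copied from the player pawn.
; It destroys itself afterward, or immediately when the roll fails.
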(event EventBeginPlay
  (bind _returnvalue (Transformation|GetActorLocation))
  (bind _returnvalue_2 (Game|Player|GetPlayerPawn 0))
  (bind _randomlocation (Class|NavigationSystemV1|GetRandomPointinNavigableRadius _returnvalue 256.0 0 0))
  (bind _returnvalue_3 (Transformation|GetActorLocation _returnvalue_2))
  (bind _z (Math|Vector|BreakVector _returnvalue_3))
  (bind _returnvalue_4 (Math|Vector|MakeVector (.x _randomlocation) (.y _randomlocation) _z))
  (bind _returnvalue_5 (Math|Transform|MakeTransform _returnvalue_4))
  (if (Math|Random|RandomBoolwithWeight 0.3)
    (Utilities|FlowControl|Delay (Math|Random|RandomFloatinRange 2.0 4.0))
    (for _index (range 0 (Math|Random|RandomIntegerinRange 0 2))
      (Game|SpawnActorfromClass "/Game/ArcCharacter/Monster/BP_MonsterCharacter.BP_MonsterCharacter_C" _returnvalue_5 "AdjustIfPossibleButAlwaysSpawn" 0 0))
    (for _index_2 (range 0 (Math|Random|RandomIntegerinRange 0 1))
      (Game|SpawnActorfromClass "/Game/ArcCharacter/RangedMonster/BP_RangedMonsterCharacter.BP_RangedMonsterCharacter_C" _returnvalue_5 "AdjustIfPossibleButAlwaysSpawn" 0 0))
    (Utilities|FlowControl|Delay 0.2))
  (Actor|DestroyActor))

(fn ConstructionScript)