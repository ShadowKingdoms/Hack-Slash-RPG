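; Blueprint function library that acts as a factory for modular armor cloth objects, from helmets and chests to cloaks and robes.
; Each function takes an Outer and a slot-specific info value, constructs the matching object class with that info, and returns the new instance.
; Left and right bracers have separate functions and classes, both initialized through a Bracers property.
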(fn ConstructHelmetCloth
  (params (Outer :type Object%20Object%20Reference) (HelmetInfo :type SROG%20Armor%20Helmets%20Structure))
  (bind _returnvalue (Game|ConstructObjectfromClass "/Game/ROG_Modular_Armor/Characters/Blueprints/Cloths/ArmorObjects/BP_BaseHelmetObject.BP_BaseHelmetObject_C" Outer HelmetInfo))
  (return _returnvalue))

(fn ConstructLeftBracersCloth
  (params (Outer :type Object%20Object%20Reference) (BracersInfo :type SROG%20Accessories%20Bracers%20Structure))
  (bind _returnvalue (Game|ConstructObjectfromClass "/Game/ROG_Modular_Armor/Characters/Blueprints/Cloths/AccessoriesObjects/BP_LeftBracerObject.BP_LeftBracerObject_C" Outer BracersInfo))
  (return _returnvalue))

(fn ConstructRightBracerCloth
  (params (Outer :type Object%20Object%20Reference) (BracerInfo :type SROG%20Accessories%20Bracers%20Structure))
  (bind _returnvalue (Game|ConstructObjectfromClass "/Game/ROG_Modular_Armor/Characters/Blueprints/Cloths/AccessoriesObjects/BP_RightBracerObject.BP_RightBracerObject_C" Outer BracerInfo))
  (return _returnvalue))

(fn ConstructChestCloth
  (params (Outer :type Object%20Object%20Reference) (ChestInfo :type SROG%20Armor%20Chests%20Structure))
  (bind _returnvalue (Game|ConstructObjectfromClass "/Game/ROG_Modular_Armor/Characters/Blueprints/Cloths/ArmorObjects/BP_BaseChestObject.BP_BaseChestObject_C" Outer ChestInfo))
  (return _returnvalue))

(fn ConstructBootsCloth
  (params (Outer :type Object%20Object%20Reference) (BootsInfo :type SROG%20Armor%20Boots%20Structure))
  (bind _returnvalue (Game|ConstructObjectfromClass "/Game/ROG_Modular_Armor/Characters/Blueprints/Cloths/ArmorObjects/BP_BaseBootsObject.BP_BaseBootsObject_C" Outer BootsInfo))
  (return _returnvalue))

(fn ConstructPantsCloth
  (params (Outer :type Object%20Object%20Reference) (PantsInfo :type SROG%20Armor%20Pants%20Structure))
  (bind _returnvalue (Game|ConstructObjectfromClass "/Game/ROG_Modular_Armor/Characters/Blueprints/Cloths/ArmorObjects/BP_BasePantsObject.BP_BasePantsObject_C" Outer PantsInfo))
  (return _returnvalue))

(fn ConstructCloakCloth
  (params (Outer :type Object%20Object%20Reference) (CloakInfo :type SROG%20Accessories%20Cloaks%20Structure))
  (bind _returnvalue (Game|ConstructObjectfromClass "/Game/ROG_Modular_Armor/Characters/Blueprints/Cloths/AccessoriesObjects/BP_CloakObject.BP_CloakObject_C" Outer CloakInfo))
  (return _returnvalue))

(fn ConstructShouldersCloth
  (params (Outer :type Object%20Object%20Reference) (ShouldersInfo :type SROG%20Accessories%20Shoulders%20Structure))
  (bind _returnvalue (Game|ConstructObjectfromClass "/Game/ROG_Modular_Armor/Characters/Blueprints/Cloths/AccessoriesObjects/BP_ShouldersObject.BP_ShouldersObject_C" Outer ShouldersInfo))
  (return _returnvalue))

(fn ConstructGlovesCloth
  (params (Outer :type Object%20Object%20Reference) (GlovesInfo :type SROG%20Accessories%20Gloves%20Structure))
  (bind _returnvalue (Game|ConstructObjectfromClass "/Game/ROG_Modular_Armor/Characters/Blueprints/Cloths/AccessoriesObjects/BP_GlovesObject.BP_GlovesObject_C" Outer GlovesInfo))
  (return _returnvalue))

(fn ConstructRobeCloth
  (params (Outer :type Object%20Object%20Reference) (RobeInfo :type SROG%20Accessories%20Robes%20Structure))
  (bind _returnvalue (Game|ConstructObjectfromClass "/Game/ROG_Modular_Armor/Characters/Blueprints/Cloths/AccessoriesObjects/BP_RobeObject.BP_RobeObject_C" Outer RobeInfo))
  (return _returnvalue))