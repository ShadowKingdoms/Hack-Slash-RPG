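; BP_Meteor is an AI ability actor that rains meteors and storms around its location and spawns a small monster spawner nearby on BeginPlay.
; Each Tick drops a meteor above a random navigable point, then randomly either spawns a storm or increments the counter.
; Only non-storm ticks count toward the randomized limit, after which the actor destroys itself following a short delay.
; A limited monster-spawning branch is left unconnected.
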(event EventBeginPlay
  (Game|SpawnActorfromClass "/Game/BluePrint/Ability/AI/SKill_2/BP_SmallMonsterSpawner.BP_SmallMonsterSpawner_C" (Math|Conversions|ToTransform(Vector) (.RandomLocation (Class|NavigationSystemV1|GetRandomPointinNavigableRadius (Transformation|GetActorLocation) 1024.0 0 0))) "Undefined" 0 0))

(event EventTick
  (params (DeltaSeconds :type Float%20%28single-precision%29))
  (bind _returnvalue (Transformation|GetActorLocation))
  (bind _randomlocation (Class|NavigationSystemV1|GetRandomPointinNavigableRadius _returnvalue 1e+03 0 0))
  (bind (_x _y _z) (Math|Vector|BreakVector _randomlocation))
  (if (> (Variables|Default|GetiMaxCount) (Variables|Default|GetiSpawnCount))
    (Game|SpawnActorfromClass "/Game/BluePrint/Ability/AI/SKill_2/BP_Unit_Meteor.BP_Unit_Meteor_C" (Math|Transform|MakeTransform (Math|Vector|MakeVector _x _y (Math|Random|RandomFloatinRange (+ _z 1e+03) (+ _z 1.5e+03))) "-90.000000,0.000000, 0") "AdjustIfPossibleButDontSpawnIfColliding" 0 0)
    (if (Math|Random|RandomBool)
      (Game|SpawnActorfromClass "/Game/BluePrint/Ability/AI/SKill_2/BP_Unit_Storm.BP_Unit_Storm_C" (Math|Conversions|ToTransform(Vector) (.RandomLocation (Class|NavigationSystemV1|GetRandomPointinNavigableRadius (Transformation|GetActorLocation) 1e+03 0 0))) "Undefined" 0 0)
      (else
        (Variables|Default|SetiSpawnCount (+ 1 (Variables|Default|GetiSpawnCount)))))
    (else
      (Utilities|FlowControl|Delay 1.0)
      (Actor|DestroyActor))))

(fn ConstructionScript
  (Variables|Default|SetiSpawnCount 0)
  (Variables|Default|SetiMaxCount (Math|Random|RandomIntegerinRange 5 10)))