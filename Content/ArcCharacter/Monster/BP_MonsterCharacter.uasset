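; Monster character that sets base stats, attaches a sword mesh component and picks a random body mesh at BeginPlay.
; Player damage rolls against the player's crit rate for double damage, spawns floating damage text and updates a temporary HP value.
; Separate events tween the HP bar toward that value by timeline, hide it, spawn an item spawner, or hide the sword and animate dynamic-material appearance before destroying the actor.
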(event Custom|Monster%20HP%20Widget%20Hidden%20Event
  (Development|SetHiddeninGame (Variables|Default|GetHPBarWidget) true false))

(event EventBeginPlay
  (Class|SkinnedMeshComponent|SetSkeletalMesh (Variables|Character|GetMesh) (Utilities|Array|Get(acopy) (Variables|Default|GetSkeletalMeshArray) (Math|Random|RandomInteger 4)) true))

(event Collision|EventActorBeginOverlap
  (params (OtherActor :type Actor%20Object%20Reference)))

(event EventDropPickupItem
  (Game|SpawnActorfromClass "/Game/BluePrint/Monster/BP_MonsterItemSpawner.BP_MonsterItemSpawner_C" (Transformation|GetActorTransform) "Undefined" 0 0))

(event EventMonsterExtinctionEffects
  (bind _mesh (Variables|Character|GetMesh))
  ;[1 1 1] Monster Death Effects
  (Development|SetHiddeninGame (Variables|Default|GetS_SwordMesh) true false)
  (bind _returnvalue (Rendering|Material|CreateDynamicMaterialInstance _mesh 0 (Rendering|Material|GetMaterial _mesh 0) "None" :!class /Script/Engine.PrimitiveComponent))
  (bind _output_get (Variables|Default|SetM_UpperApperParmRef _returnvalue))
  (bind _returnvalue_2 (Rendering|Material|CreateDynamicMaterialInstance _mesh 1 (Rendering|Material|GetMaterial _mesh 1) "None" :!class /Script/Engine.PrimitiveComponent))
  (bind _output_get_2 (Variables|Default|SetM_LowerApperParmRef _returnvalue_2))
  (bind _alpha (Timeline|Timeline Play)
    (:Update
      (Rendering|Material|SetScalarParameterValue _output_get "Apperance" _alpha :!class /Script/Engine.MaterialInstanceDynamic))
    (:Finished
      (Utilities|FlowControl|Delay 0.2)
      (Actor|DestroyActor))))

(event Game|Damage|EventAnyDamage
  (params (Damage :type Float%20%28single-precision%29) (DamageType :type Damage%20Type%20Object%20Reference) (InstigatedBy :type Controller%20Object%20Reference) (DamageCauser :type Actor%20Object%20Reference))
  (bind _aslost_arc_player_character (Utilities|Casting|CastToLostArcPlayerCharacter DamageCauser))
  (bind _returnvalue (Class|LostArcCharacterStatComponent|GetCriticalRate (Variables|/Script/LostArc.LostArcPlayerCharacter|GetStatComponent _aslost_arc_player_character)))
  ;[1 1 1] Random이 Rate 값 보다 작으면 Critical!
  (if (< (Math|Random|RandomFloatinRange 0.0 1e+02) _returnvalue)
    (bind _output_get (Variables|Default|SetDamage (* 2 Damage)))
    (CallFunction|HandleDamage _output_get true)
    (else
      (bind _output_get_2 (Variables|Default|SetDamage Damage))
      (CallFunction|HandleDamage _output_get_2 false)))
  (Variables|Default|SetMonsterTempHP (- (Variables|Default|GetMonsterHP) (Variables|Default|GetDamage))))

(event EventMonsterHPChanged
  (bind _asbp_monster_hpbar (Utilities|Casting|CastToBP_MonsterHPBar (UserInterface|GetUserWidgetObject (Variables|Default|GetHPBarWidget))))
  (if (Variables|Default|GetBar%20has%20Running)
    (Variables|Default|SetMonsterHP (- (Variables|Default|GetMonsterHP) (- (Variables|Default|GetMonsterHP) (Variables|Default|GetMonsterTempHP))))
    (bind _alpha (Timeline|HPBar%20Timeline PlayFromStart)
      (:Update
        (Progress|SetPercent (Variables|/Game/UI/Damage/BP_MonsterHPBar.BP_MonsterHPBar_C|GetProgressBar _asbp_monster_hpbar) (Math|Float|NormalizetoRange (Math|Float|Lerp (Variables|Default|GetMonsterHP) (Variables|Default|GetMonsterTempHP) _alpha) 0.0 (Variables|Default|GetMonsterMaxHP)))
        (Variables|Default|SetBar%20has%20Running true))
      (:Finished
        (Variables|Default|SetMonsterHP (Variables|Default|GetMonsterTempHP))
        (Variables|Default|SetBar%20has%20Running false)))
    (else
      (Timeline|HPBar%20Timeline PlayFromStart))))

(fn ConstructionScript
  (Variables|Default|SetMonsterStr 5.0)
  (Variables|Default|SetBasicAttackRange 2.5e+02)
  (Variables|Default|SetBasicAttackRadius 1.2e+02)
  (Variables|Default|SetMonsterDetectRadius 1024.0)
  (bind _output_get (Variables|Default|SetMonsterHP 1e+02))
  (bind _output_get_2 (Variables|Default|SetMonsterMaxHP _output_get))
  (Variables|Default|SetMonsterTempHP _output_get_2)
  (Variables|Default|SetBar%20has%20Running false)
  (Variables|Default|SetMonsterRotateSpeed 64.0)
  (bind _output_get_3 (Variables|Default|SetMonsterSpeed 3e+02))
  (Variables|/Script/Engine.CharacterMovementComponent|SetMaxWalkSpeed (Variables|Character|GetCharacterMovement) _output_get_3)
  (bind _returnvalue (AddComponent|AddSkeletalMeshComponent false))
  (bind _output_get_4 (Variables|Default|SetS_SwordMesh _returnvalue))
  (Transformation|AttachComponentToComponent _output_get_4 (Variables|Character|GetMesh) "SwordSocket" "KeepRelative" "KeepRelative" "KeepRelative" true))

(fn HandleDamage
  (params (Damage :type Float%20%28single-precision%29) (isCritical :type Boolean))
  (bind _returnvalue (Transformation|GetActorLocation))
  (bind _returnvalue_2 (Math|Random|RandomFloatinRange -4e+01 6e+01))
  (bind _returnvalue_3 (Math|Random|RandomFloatinRange 1e+02 125.0))
  (bind _returnvalue_4 (Math|Random|RandomFloatinRange -25.0 25.0))
  (bind _returnvalue_5 (+ _returnvalue (Math|Vector|MakeVector _returnvalue_4 _returnvalue_2 _returnvalue_3)))
  (if isCritical
    (bind _returnvalue_6 (Game|SpawnActorfromClass "/Game/UI/Damage/BP_FloatingCriticalTextActor.BP_FloatingCriticalTextActor_C" (Math|Transform|MakeTransform _returnvalue_5 "0, 0, 0" "1,1,1") "Undefined" 0 0))
    (Default|InitializeFunc _returnvalue_6 (Utilities|Text|ToText(Float) Damage "HalfToEven" false true 1 324 0 0))
    (else
      (bind _returnvalue_7 (Game|SpawnActorfromClass "/Game/UI/Damage/BP_FloatingTextActor.BP_FloatingTextActor_C" (Math|Transform|MakeTransform _returnvalue_5 "0, 0, 0" "1,1,1") "Undefined" 0 0))
      (Default|InitializeFunc _returnvalue_7 (Utilities|Text|ToText(Float) Damage "HalfToEven" false true 1 324 0 0)))))