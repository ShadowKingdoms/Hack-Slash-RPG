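; BP_Earth_Def_02 is a short-lived AI skill actor for an earth magic effect that damages what it hits.
; On BeginPlay it plays landing and explosion sounds, then after a brief delay activates five particle components.
; A single sphere trace at its location applies damage once to the first actor hit.
; The TL_Earth_Def timeline's event track deactivates the particles, and the actor destroys itself shortly after.
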(event EventBeginPlay
  (bind _returnvalue (Transformation|GetActorLocation))
  (bind _returnvalue_2 (Transformation|GetActorTransform))
  (bind _returnvalue_3 (Transformation|GetActorTransform))
  (bind (_location _rotation) (Math|Transform|BreakTransform _returnvalue_2))
  (bind (_location_2 _rotation_2) (Math|Transform|BreakTransform _returnvalue_3))
  (Audio|PlaySoundatLocation "/Game/Sounds/Effects/Monster/Wolf/land2-43790_1.land2-43790_1" _location _rotation 1.0 1.0 0.0 0 0 0)
  (Audio|PlaySoundatLocation "/Game/Sounds/Effects/Monster/Wolf/mixkit-war-field-explosion-1702.mixkit-war-field-explosion-1702" _location_2 _rotation_2 1.0 1.0 0.0 0 0 0)
  (Utilities|FlowControl|Delay 0.2)
  (Utilities|FlowControl|Sequence
    (:then_0
      ;[1 1 1] 1. Activates particle
      (Components|Activation|Activate (Variables|Default|GetPar_LMagic_Earth_Def_01a) false))
    (:then_1
      ;[1 1 1] sDeactivate_Particles
      (Timeline|TL_Earth_Def PlayFromStart
        (:DeActivate%20All
          ;[1 1 1] Deactivates Particle.
          (Components|Activation|Deactivate (Variables|Default|GetPar_LMagic_Earth_Def_01a))
          (Utilities|FlowControl|Delay 1.0)
          (Actor|DestroyActor))))
    (:then_2
      ;[1 1 1] Take Damage Actor
      (bind (_outhit _returnvalue_4) (Collision|SphereTraceByChannel _returnvalue _returnvalue 3e+02 "TraceTypeQuery4" false 0 "None"))
      (if _returnvalue_4
        (Game|Damage|ApplyDamage (.HitActor (Collision|BreakHitResult _outhit)) (Variables|Default|GetFDamage) 0 0)))))

(event EventTick
  (params (DeltaSeconds :type Float%20%28single-precision%29)))

(fn ConstructionScript
  (Variables|Default|SetFDamage 2e+01))