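; BP_SpawnItem is a short-lived spawner actor in the WoodBox item folder that scatters random items onto nearby navigable ground, then destroys itself.
; The construction script rolls a random spawn count.
; After a short delay on BeginPlay, the SpawnBreath macro, a delayed while-loop, spawns one random ItemTable class per pass at a random navigable point around the actor until that count is reached.
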(event EventBeginPlay
  (Utilities|FlowControl|Delay 0.5)
  (Utilities|SpawnBreath 0.3 (> (Variables|Default|GetiMaxSpawnCount) (Variables|Default|GetiSpawnCount))
    (:Loop%20Body
      (Game|SpawnActorfromClass (Utilities|Array|Get(acopy) (Variables|Default|GetItemTable) (Math|Random|RandomIntegerinRange 0 4)) (Math|Transform|MakeTransform (.RandomLocation (Class|NavigationSystemV1|GetRandomPointinNavigableRadius (Transformation|GetActorLocation) 3e+02 0 0))) "Undefined" 0 0)
      (Variables|Default|SetiSpawnCount (+ (Variables|Default|GetiSpawnCount) 1)))
    (:Exit
      (Utilities|FlowControl|Delay 0.2)
      (Actor|DestroyActor))))

(event Collision|EventActorBeginOverlap
  (params (OtherActor :type Actor%20Object%20Reference)))

(event EventTick
  (params (DeltaSeconds :type Float%20%28single-precision%29)))

(fn ConstructionScript
  (Variables|Default|SetiMaxSpawnCount (Math|Random|RandomIntegerinRange 2 5)))