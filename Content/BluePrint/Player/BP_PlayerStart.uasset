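; BP_PlayerStart is a player blueprint that checks saved inventory state in the Lost Arc game instance at BeginPlay.
; It calls DataCheck, then tests whether the instance's InventoryComponent is valid, printing a debug yes or no.
; When valid, it sets the player character's inventory and equip components and the controller's MainHUD to None rather than copying the instance's components.
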(event EventBeginPlay
  (bind _aslost_arc_game_instance (Utilities|Casting|CastToLostArcGameInstance (Game|GetGameInstance)))
  (Class|LostArcGameInstance|DataCheck _aslost_arc_game_instance)
  (if (Utilities|IsValid (Variables|/Script/LostArc.LostArcGameInstance|GetInventoryComponent _aslost_arc_game_instance))
    (Development|PrintString "yes")
    (bind _aslost_arc_player_character (Utilities|Casting|CastToLostArcPlayerCharacter (Game|Player|GetPlayerPawn 0)))
    (Variables|/Script/LostArc.LostArcPlayerCharacter|SetInventoryComponent _aslost_arc_player_character 0)
    (Variables|/Script/LostArc.LostArcPlayerCharacter|SetEquipComponent _aslost_arc_player_character 0)
    (bind _aslost_arc_player_controller (Utilities|Casting|CastToLostArcPlayerController (Game|GetPlayerController 0)))
    (Variables|/Script/LostArc.LostArcPlayerController|SetMainHUD _aslost_arc_player_controller 0)
    (else
      (Development|PrintString "No"))))

(event EventTick
  (params (DeltaSeconds :type Float%20%28single-precision%29)))

(fn ConstructionScript)