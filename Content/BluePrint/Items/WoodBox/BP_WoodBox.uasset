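; Wooden item box that the player can open to release items.
; On overlap it registers itself in the player's AbilityComponent as ItemBoxPtr and prints a debug string, then clears that pointer when the overlap ends.
; SpawnItems, which is not called within this Blueprint, spawns an opening effect and a BP_BoxItemSpawner at the box's location, then sets a short lifespan so the box removes itself.
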(event EventBeginPlay)

(event Collision|EventActorBeginOverlap
  (params (OtherActor :type Actor%20Object%20Reference))
  (bind _asbp_lost_arc_player_character (Utilities|Casting|CastToBP_LostArcPlayerCharacter OtherActor))
  (Variables|/Script/LostArc.LostArcCharacterAbilityComponent|SetItemBoxPtr (Variables|/Script/LostArc.LostArcPlayerCharacter|GetAbilityComponent _asbp_lost_arc_player_character) self)
  (Development|PrintString "ItemBox" true true "(R=1.000000,G=0.963152,B=0.086832,A=1.000000)"))

(event EventTick
  (params (DeltaSeconds :type Float%20%28single-precision%29)))

(event Collision|EventActorEndOverlap
  (params (OtherActor :type Actor%20Object%20Reference))
  (bind _asbp_lost_arc_player_character (Utilities|Casting|CastToBP_LostArcPlayerCharacter OtherActor))
  (Variables|/Script/LostArc.LostArcCharacterAbilityComponent|SetItemBoxPtr (Variables|/Script/LostArc.LostArcPlayerCharacter|GetAbilityComponent _asbp_lost_arc_player_character) 0))

(fn ConstructionScript)

(fn SpawnItems
  (bind _returnvalue (Transformation|GetActorLocation))
  (bind _returnvalue_2 (Math|Transform|MakeTransform _returnvalue))
  (Game|SpawnActorfromClass "/Game/BluePrint/Items/WoodBox/BP_WoodBox_OpenEffect.BP_WoodBox_OpenEffect_C" _returnvalue_2 "Undefined" 0 0)
  (Game|SpawnActorfromClass "/Game/BluePrint/Items/WoodBox/BP_BoxItemSpawner.BP_BoxItemSpawner_C" _returnvalue_2 "Undefined" 0 0)
  (Actor|SetLifeSpan 0.5))