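; BP_BaseClothObject is the base object for a wearable clothing piece in the modular armor system, exposing its type and owner mesh tag.
; Mesh, morph target and body slot getters are empty here, apparently for child classes to override.
; Add and remove functions message the outer object to set or clear the tagged mesh, then add or remove any morph and body slot targets.
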(fn GetMorphTargets
  (return 0))

(fn GetType
  (return (Variables|Default|GetClothType)))

(fn GetMeshTagonOwner
  (return (Variables|Default|GetClothTagOnOwner)))

(fn GetMesh
  (return 0))

(fn AddClothtoOwner
  (Class|BPIClothInterface|SetClothMeshbyTag(Message) (Utilities|GetOuterObject self) (CallFunction|GetMesh) (CallFunction|GetMeshTagonOwner))
  (Utilities|FlowControl|Sequence
    (:then_0
      (if (> (Utilities|Array|Length (CallFunction|GetMorphTargets)) 0)
        (Class|BPIClothInterface|AddMorphTargets(Message) (Utilities|GetOuterObject self) (CallFunction|GetMorphTargets))))
    (:then_1
      (if (> (Utilities|Array|Length (CallFunction|GetBodySlotsTargets)) 0)
        (Class|BPIClothInterface|AddBodySlotsTargets(Message) (Utilities|GetOuterObject self) (CallFunction|GetBodySlotsTargets))))))

(fn RemoveClothfromOwner
  (Class|BPIClothInterface|SetClothMeshbyTag(Message) (Utilities|GetOuterObject self) 0 (CallFunction|GetMeshTagonOwner))
  (Utilities|FlowControl|Sequence
    (:then_0
      (if (> (Utilities|Array|Length (CallFunction|GetMorphTargets)) 0)
        (Class|BPIClothInterface|RemoveMorphTargets(Message) (Utilities|GetOuterObject self) (CallFunction|GetMorphTargets))))
    (:then_1
      (if (> (Utilities|Array|Length (CallFunction|GetBodySlotsTargets)) 0)
        (Class|BPIClothInterface|RemoveBodySlotsTargets(Message) (Utilities|GetOuterObject self) (CallFunction|GetBodySlotsTargets))))))

(fn GetBodySlotsTargets
  (return 0))