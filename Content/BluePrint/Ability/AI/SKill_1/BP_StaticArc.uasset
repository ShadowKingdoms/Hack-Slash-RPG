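; Short-lived arc visual for an AI skill that sweeps in a randomly chosen direction, then removes itself.
; On BeginPlay it creates dynamic materials for Circle and CircleRvs, setting scalar parameters to shape each arc.
; A random bool reveals one of them and plays its matching timeline, which drives the yaw of CircleRoot.
; The actor destroys itself shortly after the timeline finishes.
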(event EventBeginPlay
  (Utilities|FlowControl|Sequence
    (:then_0
      ;[1 1 1] Construct Material Instances
      (bind _returnvalue (Rendering|Material|CreateDynamicMaterialInstance (Variables|디폴트|GetCircle) :!class /Script/Engine.DecalComponent))
      (bind _output_get (Variables|디폴트|SetCircleRef _returnvalue))
      (Rendering|Material|SetScalarParameterValue _output_get "Circum1Area0" 0.0 :!class /Script/Engine.MaterialInstanceDynamic)
      (Rendering|Material|SetScalarParameterValue _output_get "RadianValue" 0.125 :!class /Script/Engine.MaterialInstanceDynamic))
    (:then_1
      (bind _returnvalue_2 (Rendering|Material|CreateDynamicMaterialInstance (Variables|Default|GetCircleRvs) :!class /Script/Engine.DecalComponent))
      (bind _output_get_2 (Variables|디폴트|SetCircleRvsRef _returnvalue_2))
      (Rendering|Material|SetScalarParameterValue _output_get_2 "Circum1Area0" 0.0 :!class /Script/Engine.MaterialInstanceDynamic)
      (Rendering|Material|SetScalarParameterValue _returnvalue_2 "RadianValue" 0.125 :!class /Script/Engine.MaterialInstanceDynamic))
    (:then_2
      (if (Math|Random|RandomBool)
        ;[1 1 1] Rotate to Circle L
        (Rendering|SetVisibility (Variables|디폴트|GetCircle) true false)
        (bind _newtrack (Timeline|RoatateTickScale Play)
          (:Update
            (Transformation|SetRelativeRotation (Variables|Default|GetCircleRoot) (Math|Rotator|MakeRotator 0.0 0.0 _newtrack) false false))
          (:Finished
            (Utilities|FlowControl|Delay 0.2)
            (Actor|DestroyActor)))
        (else
          ;[1 1 1] Rotate to Circle L
          (Rendering|SetVisibility (Variables|Default|GetCircleRvs) true false)
          (bind _rvstrack (Timeline|RotateTickScale_Rvs Play)
            (:Update
              (Transformation|SetRelativeRotation (Variables|Default|GetCircleRoot) (Math|Rotator|MakeRotator 0.0 0.0 _rvstrack) false false))
            (:Finished
              (Utilities|FlowControl|Delay 0.2)
              (Actor|DestroyActor))))))))

(fn ConstructionScript)