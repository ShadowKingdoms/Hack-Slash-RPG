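; BP_Shield_Aqua is a temporary water shield actor that follows player 0 by copying its location every Tick.
; On BeginPlay it activates its particle, and one timeline scales it up from zero.
; During that timeline, a half-second Delay on Update gates HitDetection calls on the player's MeleeSkill2 ability.
; A second timeline then shrinks the particle, with a one-second Delay from its Update leading to DestroyActor.
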(event EventTick
  (params (DeltaSeconds :type Float%20%28single-precision%29))
  ;[1 1 1] SetActorLocation Tick
  (Transformation|SetActorLocation (.Location (Math|Transform|BreakTransform (Transformation|GetActorTransform (Game|GetPlayerCharacter 0)))) false false))

(event EventBeginPlay
  (bind _par_lmagic_aqua_def_01 (Variables|Default|GetPar_LMagic_Aqua_Def_01))
  ;[1 1 1] Scale Lerp
  (Components|Activation|Activate _par_lmagic_aqua_def_01 false)
  (bind _aqua_def_time (Timeline|TL_Aqua_On PlayFromStart)
    (:Update
      (Transformation|SetRelativeScale3D _par_lmagic_aqua_def_01 (Math|Vector|Lerp(Vector) "0, 0, 0" "1.000000,1.000000,1.000000" _aqua_def_time))
      (Utilities|FlowControl|Delay 0.5)
      ;[1 1 1] Hit Detection
      (bind _aslost_arc_player_character (Utilities|Casting|CastToLostArcPlayerCharacter (Game|GetPlayerCharacter 0)))
      (bind _returnvalue (Class|LostArcCharacterAbilityComponent|GetAbilities (Variables|/Script/LostArc.LostArcPlayerCharacter|GetAbilityComponent _aslost_arc_player_character) "MeleeSkill_2"))
      (Class|LostArcSkillBase|HitDetection _returnvalue _aslost_arc_player_character))
    (:Finished
      (bind _aqua_def_time_2 (Timeline|TL_Aqua_Off Play)
        (:Update
          (Transformation|SetRelativeScale3D _par_lmagic_aqua_def_01 (Math|Vector|Lerp(Vector) "1.000000,1.000000,1.000000" "0, 0, 0" _aqua_def_time_2))
          (Utilities|FlowControl|Delay 1.0)
          (Actor|DestroyActor))))))

(fn ConstructionScript)