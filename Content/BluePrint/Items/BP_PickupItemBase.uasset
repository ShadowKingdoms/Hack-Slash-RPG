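; Base Blueprint for pickup items that the player collects into the inventory by overlapping them.
; Collision stays off from construction until shortly after BeginPlay, then an overlap by LostArcPlayerCharacter checks the inventory for an empty slot.
; On success it plays a sound, hides the light, and a timeline shrinks and pulls the mesh toward the player.
; When the timeline finishes, it adds the named item and destroys itself.
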(event Custom|AnimateCollection
  (bind _staticmesh (Variables|Default|GetStaticMesh))
  (Audio|PlaySound2D "/Game/Sounds/Effects/Item/ItemRootingEffect.ItemRootingEffect" 1.0 1.0 0.0 "/Game/Sounds/Effects/Item/ItemRootingConcurrency.ItemRootingConcurrency" 0)
  (bind _alpha (Timeline|Animate Play)
    (:Update
      (Transformation|SetRelativeScale3D _staticmesh (Math|Vector|Lerp(Vector) (Transformation|GetWorldScale (Variables|Default|GetStaticMesh)) "0, 0, 0" _alpha)) ; Animate mesh scale effect
      (Transformation|SetWorldLocation _staticmesh (Math|Vector|Lerp(Vector) (Transformation|GetWorldLocation (Variables|Default|GetStaticMesh)) (Transformation|GetActorLocation (Game|Player|GetPlayerPawn 0)) _alpha) false true) ; Smooth move mesh to player position
    )
    (:Finished
      (Class|LostArcInventoryComponent|AddPickupItem (Variables|/Script/LostArc.LostArcPlayerCharacter|GetInventoryComponent (Variables|Default|GetPlayerRef)) (Variables|Default|GetFPickupItemName) 1)
      (Utilities|FlowControl|Delay 0.1)
      (Actor|DestroyActor))))

(event EventBeginPlay
  (Utilities|FlowControl|Delay 2.0)
  (Collision|SetCollisionEnabled (Variables|Default|GetCollision) "QueryOnly"))

(event Collision|EventActorBeginOverlap
  (params (OtherActor :type Actor%20Object%20Reference))
  (bind _aslost_arc_player_character (Utilities|Casting|CastToLostArcPlayerCharacter OtherActor))
  (Variables|Default|SetPlayerRef _aslost_arc_player_character)
  (bind _returnvalue (Class|LostArcInventoryComponent|InventorySlotEmptyCheck (Variables|/Script/LostArc.LostArcPlayerCharacter|GetInventoryComponent (Variables|Default|GetPlayerRef))))
  (if _returnvalue
    (CallFunction|AnimateCollection)
    (Development|SetHiddeninGame (Variables|Default|GetPointLight) true false)
    (Collision|SetCollisionEnabled (Variables|Default|GetCollision) "NoCollision")))

(event EventTick
  (params (DeltaSeconds :type Float%20%28single-precision%29)))

(fn ConstructionScript
  (Collision|SetCollisionEnabled (Variables|Default|GetCollision) "NoCollision"))