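; Small monster spawner that scatters a small random number of actors around itself at level start, then removes itself.
; On BeginPlay, two randomly sized loops spawn actors near navigable points within a fixed radius, raised above the ground, adjusting for collisions but always spawning.
; Each X, Y and Z comes from a separate random-point query, so positions can mix different points.
; After a short delay the spawner destroys itself.
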(event EventBeginPlay
  (bind _returnvalue (Transformation|GetActorLocation))
  (bind _randomlocation (Class|NavigationSystemV1|GetRandomPointinNavigableRadius _returnvalue 384.0 0 0))
  (bind _returnvalue_2 (+ (.z _randomlocation) 512.0))
  (bind _returnvalue_3 (Math|Vector|MakeVector (.x _randomlocation) (.y _randomlocation) _returnvalue_2))
  (bind _returnvalue_4 (Math|Transform|MakeTransform _returnvalue_3))
  (for _index (range 0 (Math|Random|RandomIntegerinRange 0 1))
    (Game|SpawnActorfromClass "/Game/ArcCharacter/Monster/BP_MonsterCharacter.BP_MonsterCharacter_C" _returnvalue_4 "AdjustIfPossibleButAlwaysSpawn" 0 0))
  (for _index_2 (range 0 (Math|Random|RandomIntegerinRange 0 1))
    (Game|SpawnActorfromClass "/Game/ArcCharacter/RangedMonster/BP_RangedMonsterCharacter.BP_RangedMonsterCharacter_C" _returnvalue_4 "AdjustIfPossibleButAlwaysSpawn" 0 0))
  (Utilities|FlowControl|Delay 0.2)
  (Actor|DestroyActor))

(fn ConstructionScript)