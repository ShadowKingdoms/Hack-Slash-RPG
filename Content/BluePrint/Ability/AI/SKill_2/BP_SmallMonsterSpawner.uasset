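; BP_SmallMonsterSpawner is a one-shot spawner that may release a small group of melee and ranged monsters around its location.
; On BeginPlay it makes a weighted random roll, and on success waits a random few seconds before spawning.
; Random counts of BP_MonsterCharacter and BP_RangedMonsterCharacter appear at random navmesh points within a small radius.
; It destroys itself afterwards, or immediately if the roll fails.
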(event EventBeginPlay
  (bind _returnvalue (Transformation|GetActorLocation))
  (bind _randomlocation (Class|NavigationSystemV1|GetRandomPointinNavigableRadius _returnvalue 256.0 0 0))
  (bind _returnvalue_2 (Math|Transform|MakeTransform _randomlocation))
  (if (Math|Random|RandomBoolwithWeight 0.3)
    (Utilities|FlowControl|Delay (Math|Random|RandomFloatinRange 2.0 4.0))
    (for _index (range 0 (Math|Random|RandomIntegerinRange 0 3))
      (Game|SpawnActorfromClass "/Game/ArcCharacter/Monster/BP_MonsterCharacter.BP_MonsterCharacter_C" _returnvalue_2 "Undefined" 0 0))
    (for _index_2 (range 0 (Math|Random|RandomIntegerinRange 0 2))
      (Game|SpawnActorfromClass "/Game/ArcCharacter/RangedMonster/BP_RangedMonsterCharacter.BP_RangedMonsterCharacter_C" _returnvalue_2 "Undefined" 0 0))
    (Utilities|FlowControl|Delay 0.2))
  (Actor|DestroyActor))

(fn ConstructionScript)