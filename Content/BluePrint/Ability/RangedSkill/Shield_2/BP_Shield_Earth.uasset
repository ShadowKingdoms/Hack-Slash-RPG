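; BP_Shield_Earth is a self-destroying earth shield effect actor for a player ability.
; On BeginPlay it activates five earth particle components, plays a meteor impact sound and starts a timeline.
; After a short delay it calls HitDetection on the MeleeSkill4 ability from the player character's AbilityComponent.
; A timeline event later deactivates the particles, and the actor destroys itself after a further delay.
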(event EventBeginPlay
  (Utilities|FlowControl|Sequence
    (:then_0
      ;[1 1 1] 1. Activates particle
      (Components|Activation|Activate (Variables|Default|GetPar_LMagic_Earth_Def_01a) false))
    (:then_1
      ;[1 1 1] Deactivate_Particles
      (Timeline|TL_Earth_Def PlayFromStart
        (:DeActivate%20All
          ;[1 1 1] Deactivates Particle.
          (Components|Activation|Deactivate (Variables|Default|GetPar_LMagic_Earth_Def_01a))
          (Utilities|FlowControl|Delay 2.0)
          (Actor|DestroyActor))))
    (:then_2
      (Audio|PlaySoundatLocation "/Game/Sounds/Abilities/A_Ability_MeteorImpact_Cue.A_Ability_MeteorImpact_Cue" (Transformation|GetActorLocation) "0, 0, 0" 1.0 1.0 0.0 0 0 0)
      (Utilities|FlowControl|Delay 0.1)
      ;[1 1 1] Hit Detection
      (bind _aslost_arc_player_character (Utilities|Casting|CastToLostArcPlayerCharacter (Game|GetPlayerCharacter 0)))
      (bind _returnvalue (Class|LostArcCharacterAbilityComponent|GetAbilities (Variables|/Script/LostArc.LostArcPlayerCharacter|GetAbilityComponent _aslost_arc_player_character) "MeleeSkill_4"))
      (Class|LostArcSkillBase|HitDetection _returnvalue _aslost_arc_player_character))))

(fn ConstructionScript)