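; BP_Circular_Static is a static circular-sector ability indicator.
; On BeginPlay it creates a dynamic material instance on its Area component and sets fixed scalar parameters for area mode, radian and area value, so the shape does not animate.
; Unconnected leftover logic would set up a Circum outline material and play a timeline that animates the area value before destroying the actor.
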(event EventBeginPlay
  (Utilities|FlowControl|Sequence
    (:then_1
      ;[1 1 1] Construct Material Instances
      (bind _returnvalue (Rendering|Material|CreateDynamicMaterialInstance (Variables|컴포넌트|GetArea) :!class /Script/Engine.DecalComponent))
      (bind _output_get (Variables|Default|SetAreaRef _returnvalue))
      (Rendering|Material|SetScalarParameterValue _output_get "Circum1Area0" 0.0 :!class /Script/Engine.MaterialInstanceDynamic))
    (:then_2
      (Rendering|Material|SetScalarParameterValue (Variables|Default|GetAreaRef) "RadianValue" 0.2 :!class /Script/Engine.MaterialInstanceDynamic)
      (Rendering|Material|SetScalarParameterValue (Variables|Default|GetAreaRef) "AreaValue" 0.5 :!class /Script/Engine.MaterialInstanceDynamic))))

(fn ConstructionScript)