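; BP_Unit_Storm is a lightning storm actor, apparently an AI skill effect, that deals periodic area damage where it stands.
; On BeginPlay it plays thunder, then after a short delay activates the lightning particle, a timeline and a damage loop.
; The Hit Delay macro repeatedly fires a single-hit sphere trace, damaging one actor per tick.
; The timeline's event deactivates the particle and destroys the actor, ending the otherwise endless loop.
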(event EventBeginPlay
  (bind _returnvalue (Transformation|GetActorLocation))
  (bind _returnvalue_2 (Transformation|GetActorTransform))
  (bind (_location _rotation) (Math|Transform|BreakTransform _returnvalue_2))
  (Audio|PlaySoundatLocation "/Game/Sounds/Effects/Monster/Wolf/mixkit-cinematic-thunder-1283-cut.mixkit-cinematic-thunder-1283-cut" _location _rotation 1.0 1.0 0.0 0 "/Game/Sounds/Effects/Monster/Wolf/ThunderSoundConcurrency.ThunderSoundConcurrency" 0)
  (Utilities|FlowControl|Delay 0.2)
  (Utilities|FlowControl|Sequence
    (:then_0
      ;[1 1 1] 1. Activates particle
      (Components|Activation|Activate (Variables|Default|GetPar_Lightning) false))
    (:then_1
      ;[1 1 1] Deactivate_Particles
      (Timeline|TL_Earth_Def PlayFromStart
        (:DeActivate%20All
          (Components|Activation|Deactivate (Variables|Default|GetPar_Lightning))
          (Utilities|FlowControl|Delay 0.1)
          (Actor|DestroyActor))))
    (:then_2
      ;[1 1 1] Tick Damage Actor
      (Utilities|HitDelay 0.5 true
        (:Loop%20Body
          (bind (_outhit _returnvalue_3) (Collision|SphereTraceByChannel _returnvalue _returnvalue 3e+02 "TraceTypeQuery4" false 0 "None"))
          (if _returnvalue_3
            (Game|Damage|ApplyDamage (.HitActor (Collision|BreakHitResult _outhit)) (Variables|Default|GetFTickDamage) 0 0)))))))

(fn ConstructionScript
  (Variables|Default|SetFTickDamage 5.0))