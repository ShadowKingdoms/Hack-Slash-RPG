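; BP_RobeObject is a cloth accessory object that describes a robe for the modular armor character system.
; GetMesh returns the robe mesh stored in its RobeInfo struct.
; GetBodySlotsTargets adds the arms body slot to the target list for one robe type and returns that list.
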(fn GetMesh
  (return (Utilities|Struct|BreakSROG_Accessories_Robes (Variables|Default|GetRobeInfo))))

(fn GetBodySlotsTargets
  (Utilities|FlowControl|Sequence
    (:then_0
      (if (Utilities|Enum|Equal(Enum) (.RobeType (Utilities|Struct|BreakSROG_Accessories_Robes (Variables|Default|GetRobeInfo))) "NewEnumerator1")
        (Utilities|Array|Add (LocalVariables|Get_Targets) "BODY_ARMS")))
    (:then_1
      (return (LocalVariables|Get_Targets)))))