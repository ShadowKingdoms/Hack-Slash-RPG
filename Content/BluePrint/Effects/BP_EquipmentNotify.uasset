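; BP_EquipmentNotify is a short-lived actor that shows an on-screen equipment notification.
; NotifyConstruct creates a BP_EquipmentUI widget for the first player, passing a title and numeric value as text, and adds it to the viewport.
; The LifeCycle timeline starts at BeginPlay and removes the widget when finished, while the construction script sets a brief lifespan so the actor destroys itself.
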(event EventBeginPlay
  (Timeline|LifeCycle Play
    (:Finished
      (Widget|RemovefromParent (Variables|Default|GetWidget)))))

(event Collision|EventActorBeginOverlap
  (params (OtherActor :type Actor%20Object%20Reference)))

(event EventTick
  (params (DeltaSeconds :type Float%20%28single-precision%29)))

(fn ConstructionScript
  (Actor|SetLifeSpan 2.5))

(fn NotifyConstruct
  (params (T :type String) (V :type Float%20%28single-precision%29))
  (bind _returnvalue (UserInterface|CreateWidget "/Game/BluePrint/Effects/BP_EquipmentUI.BP_EquipmentUI_C" (Game|GetPlayerController 0) (Utilities|Text|ToText(String) T) (Utilities|Text|ToText(Float) V "HalfToEven")))
  (bind _output_get (Variables|Default|SetWidget _returnvalue))
  (UserInterface|Viewport|AddtoViewport _output_get 0))