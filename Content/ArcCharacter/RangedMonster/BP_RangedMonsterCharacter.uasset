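; Ranged monster character whose construction script sets its attack range, detection radius, health and movement stats.
; HP change events update a BP_MonsterHPBar widget, and the drop event spawns a BP_MonsterItemSpawner at the monster's transform.
; The extinction event hides the bar, animates an "Apperance" parameter on two dynamic mesh materials through a timeline, then destroys the actor.
; Any actor overlap swaps the skeletal mesh to a random array entry.
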(event EventBeginPlay)

(event Collision|EventActorBeginOverlap
  (params (OtherActor :type Actor%20Object%20Reference))
  (Class|SkinnedMeshComponent|SetSkeletalMesh (Variables|Character|GetMesh) (Utilities|Array|Get(acopy) (Variables|Default|GetSkeletalMeshArray) (Math|Random|RandomInteger 3)) true))

(event EventTick
  (params (DeltaSeconds :type Float%20%28single-precision%29)))

(event EventDropPickupItem
  (Game|SpawnActorfromClass "/Game/BluePrint/Monster/BP_MonsterItemSpawner.BP_MonsterItemSpawner_C" (Transformation|GetActorTransform) "Undefined" 0 0))

(event EventMonsterExtinctionEffects
  (bind _mesh (Variables|Character|GetMesh))
  (Development|SetHiddeninGame (Variables|Default|GetHPBarWidget) true false)
  (bind _returnvalue (Rendering|Material|CreateDynamicMaterialInstance _mesh 0 (Rendering|Material|GetMaterial _mesh 0) "None" :!class /Script/Engine.PrimitiveComponent))
  (bind _output_get (Variables|Default|SetM_UpperApperParmRef _returnvalue))
  (bind _returnvalue_2 (Rendering|Material|CreateDynamicMaterialInstance _mesh 1 (Rendering|Material|GetMaterial _mesh 1) "None" :!class /Script/Engine.PrimitiveComponent))
  (bind _output_get_2 (Variables|Default|SetM_LowerApperParmRef _returnvalue_2))
  (bind _alpha (Timeline|Timeline Play)
    (:Update
      (Rendering|Material|SetScalarParameterValue _output_get "Apperance" _alpha :!class /Script/Engine.MaterialInstanceDynamic))
    (:Finished
      (Utilities|FlowControl|Delay 0.2)
      (Actor|DestroyActor))))

(event EventMonsterHPChanged
  (bind _asbp_monster_hpbar (Utilities|Casting|CastToBP_MonsterHPBar (UserInterface|GetUserWidgetObject (Variables|Default|GetHPBarWidget))))
  (Default|SetPercent _asbp_monster_hpbar (/ (Variables|Default|GetMonsterHP) (Variables|Default|GetMonsterMaxHP))))

(fn ConstructionScript
  (Variables|Default|SetBasicAttackRange 8e+02)
  (Variables|Default|SetMonsterDetectRadius 1536.0)
  (bind _output_get (Variables|Default|SetMonsterHP 1e+02))
  (Variables|Default|SetMonsterMaxHP _output_get)
  (Variables|Default|SetMonsterRotateSpeed 64.0)
  (bind _output_get_2 (Variables|Default|SetMonsterSpeed 2e+02))
  (Variables|/Script/Engine.CharacterMovementComponent|SetMaxWalkSpeed (Variables|Character|GetCharacterMovement) _output_get_2))