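; BP_LostArcPlayerCharacter is the Greystone player character Blueprint, handling feedback for damage, consumables and equipment, plus level music at BeginPlay.
; Damage spawns floating text and an impact sound, while potion use spawns an effect actor with a sound.
; Equipment changes replace any existing notify actor with a new one, and a rooting event plays an interaction montage.
; The construction script initializes MaxHP from the StatComponent's current HP.
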(event EventBeginPlay
  (Audio|PlaySound2D "/Game/Sounds/Music/MainSoundtrack_Cue.MainSoundtrack_Cue" 1.0 1.0 0.0 "/Game/Sounds/Music/BGMConcurrency.BGMConcurrency" 0))

(event EventCharacterConsumeEffect
  (Game|SpawnActorfromClass "/Game/BluePrint/Effects/BP_PotionConsumeEffect.BP_PotionConsumeEffect_C" (Transformation|GetActorTransform) "Undefined" 0 0)
  (Audio|PlaySound2D "/Game/Sounds/Character/A_Character_Potion_Cue.A_Character_Potion_Cue" 1.0 1.0 0.0 0 0))

(event EventOnPlayerTakeDamage
  (params (Damage :type Float%20%28single-precision%29))
  (bind _returnvalue (Transformation|GetActorTransform))
  (bind (_location _rotation) (Math|Transform|BreakTransform _returnvalue))
  (bind _returnvalue_2 (Game|SpawnActorfromClass "/Game/UI/Damage/BP_PlayerFloatingTextActor.BP_PlayerFloatingTextActor_C" (Math|Transform|MakeTransform (|CalculatieLocation) "0, 0, 0" "1,1,1") "Undefined" 0 0))
  (Default|InitializeFunc _returnvalue_2 (Utilities|Text|ToText(Float) Damage "HalfToEven" false true 1 324 0 0))
  (Audio|PlaySoundatLocation "/Game/Sounds/Creatures/Guardian/A_Guardian_ImpactL_Cue.A_Guardian_ImpactL_Cue" _location _rotation 1.0 1.0 0.0 0 "/Game/Sounds/Effects/CharacterHit/CharacterHitSoundConcurrency.CharacterHitSoundConcurrency" 0))

(event EventCharacterEquipmentEffect
  (params (Name :type String) (Value :type Float%20%28single-precision%29))
  (Utilities|IsValid (Variables|Default|GetEquipmentNotfiy)
    (:Is%20Valid
      (Default|DestoryActor (Variables|Default|GetEquipmentNotfiy)))
    (:Is%20Not%20Valid
      _))
  (bind _returnvalue (Game|SpawnActorfromClass "/Game/BluePrint/Effects/BP_EquipmentNotify.BP_EquipmentNotify_C" (Transformation|GetActorTransform) "Undefined" 0 0))
  (bind _output_get (Variables|Default|SetEquipmentNotfiy _returnvalue))
  (Default|NotifyConstruct _output_get Name Value))

(event EventPlayRootingAnimation
  (Animation|PlayAnimMontage "/Game/ArcCharacter/Greystone/Ability/Greystone_Interaction_Cut_Montage.Greystone_Interaction_Cut_Montage" 1.0 "None"))

(fn ConstructionScript
  (Utilities|FlowControl|Sequence
    (:then_0
      (bind _returnvalue (Class|LostArcCharacterStatComponent|GetCurrentAttributeValue (Variables|Default|GetStatComponent) "HP"))
      (Variables|Default|SetMax%20HP _returnvalue))))